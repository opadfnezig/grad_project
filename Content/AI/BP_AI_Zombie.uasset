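; Zombie AI character that activates when pawn sensing sees a pawn and melees with a montage-driven attack.
; Attack is gated by CanAttack, waits into the montage, then sphere-traces between two attack sockets and applies damage to whatever it hits.
; Incoming damage lowers NPCStats health; at zero or below it spawns a health pack nearby and destroys itself.
; Debug prints and trace drawing remain in place.
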(event `self.PawnSensing.OnSeePawn`
  (params (Pawn :type "Pawn Object Reference"))
  (`self.ActivateAI` self))

(event `self.ReceiveAnyDamage`
  (params (Damage :type "Float (single-precision)") (DamageType :type "DamageType Object Reference") (InstigatedBy :type "Controller Object Reference") (DamageCauser :type "Actor Object Reference"))
  (bind (_returnvalue_x _returnvalue_y _returnvalue_z) (`KismetMathLibrary.BreakVector` (`self.K2_GetActorLocation` (`ActorComponent.GetOwner` (`self.PawnSensing`)))))
  (if (> (`/Game/AI/NPC_Stats.Health` (`self.NPC_Stats`)) 0.0)
    (bind _output_get (set `/Game/AI/NPC_Stats.Health` (- (`/Game/AI/NPC_Stats.Health` (`self.NPC_Stats`)) Damage) (`self.NPC_Stats`)))
    (`KismetSystemLibrary.PrintString` (`KismetStringLibrary.Conv_DoubleToString` _output_get))
    (if (<= _output_get 0.0)
      (`|SpawnActorFromClass` "/Game/Blueprints/Pickup/BP_HealthPack.BP_HealthPack_C" (`KismetMathLibrary.MakeTransform` (`KismetMathLibrary.MakeVector` (- _returnvalue_x 100.0) _returnvalue_y _returnvalue_z)) "Undefined" "OverrideRootScale" null null)
      (`self.K2_DestroyActor`))))

(event `AttackEvent`
  (if (`self.bCanAttack`)
    (set `self.bCanAttack` false)
    (`self.PlayAnimMontage` (`CharacterMovementComponent.GetCharacterOwner` (`self.CharacterMovement`)) "/Game/Animations/Attack_Montage.Attack_Montage" 1.0 "None")
    (`KismetSystemLibrary.Delay` 0.7)
    (bind _outhit (`KismetSystemLibrary.SphereTraceSingle` :`Start` (`SceneComponent.GetSocketLocation` (`self.StartAttackPos`) "None") :`End` (`SceneComponent.GetSocketLocation` (`self.EndAttackPos`) "None") :`Radius` 10.0 :`TraceChannel` "TraceTypeQuery1" :`DrawDebugType` "ForDuration"))
    (`KismetSystemLibrary.PrintString` (`KismetSystemLibrary.GetObjectName` (`.HitActor` (`GameplayStatics.BreakHitResult` _outhit))))
    (`GameplayStatics.ApplyDamage` (`.HitActor` (`GameplayStatics.BreakHitResult` _outhit)) 15.0)
    (`KismetSystemLibrary.Delay` 0.3)
    (set `self.bCanAttack` true)))

(fn `Attack`
  (`self.AttackEvent`))

(fn `UserConstructionScript`)