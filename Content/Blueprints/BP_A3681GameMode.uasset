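; Game mode that opens the game on a main menu and provides a function to hand control to the player character.
; On BeginPlay it creates and displays the MainMenu widget, shows the mouse cursor, then unpossesses the first player controller after a short delay.
; SpawnPlayer finds the existing BP_ThirdPersonCharacter in the level, possesses it and adds the player HUD, without spawning a new actor.
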(event `self.ReceiveBeginPlay`
  (bind _returnvalue (`|GenericCreateObject` self "/Game/Widgets/MainMenu.MainMenu_C"))
  (bind _output_get (set `self.MainMenu` _returnvalue))
  (`UserWidget.AddToViewport` _returnvalue 0)
  (`UserWidget.AddToViewport` _output_get 0)
  (set `PlayerController.bShowMouseCursor` true (`GameplayStatics.GetPlayerController` 0))
  (`KismetSystemLibrary.Delay` 0.5)
  (`Controller.UnPossess` (`GameplayStatics.GetPlayerController` 0)))

(fn `SpawnPlayer`
  (bind _returnvalue (`GameplayStatics.GetPlayerController` 0))
  (bind _returnvalue_2 (`GameplayStatics.GetActorOfClass` "/Game/StarterContent/ThirdPerson/Blueprints/BP_ThirdPersonCharacter.BP_ThirdPersonCharacter_C"))
  (`Controller.Possess` _returnvalue _returnvalue_2)
  (bind _returnvalue_3 (`|GenericCreateObject` _returnvalue "/Game/Widgets/WP_PlayerHUD.WP_PlayerHUD_C"))
  (`UserWidget.AddToViewport` _returnvalue_3 0))

(fn `UserConstructionScript`)