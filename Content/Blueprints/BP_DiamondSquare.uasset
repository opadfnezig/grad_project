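; Procedural terrain actor that builds a random diamond-square landscape as a collidable ProceduralMesh with a moss material.
; GenerateLandscape clears and rebuilds the mesh; BeginPlay and the construction script do nothing.
; GENERATOR creates the grid, seeds corner heights, then subdivides squares iteratively through swapped index arrays.
; DIAMOND displaces midpoints and still-zero edge points, halving the random range on every call rather than every pass.
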(event `self.ReceiveBeginPlay`)

(fn `DIAMOND`
  (params (SQ_A :type Integer) (SQ_B :type Integer) (SQ_C :type Integer) (SQ_D :type Integer))
  (returns (A :type Integer) (B :type Integer) (C :type Integer) (D :type Integer) (MID :type Integer) (Left :type Integer) (Top :type Integer) (Right :type Integer) (Bottom :type Integer))
  (locals (L_SQ_A :type Integer) (L_SQ_B :type Integer) (L_SQ_C :type Integer) (L_SQ_D :type Integer) (L_MID :type Integer) (`L:_DMD_Left` :type Integer) (L_DMD_Top :type Integer) (L_DMD_Right :type Integer) (L_DMD_Bottom :type Integer) (V_MID :type "Float (double-precision)"))
  (bind _vertex (`self.VERTEX`))
  (bind _spec (`self.SPEC`))
  (bind _l_mid (`local.L_MID`))
  (bind _vertex_2 (`self.VERTEX`))
  (bind _vertex_3 (`self.VERTEX`))
  (bind _vertex_4 (`self.VERTEX`))
  (bind _vertex_5 (`self.VERTEX`))
  (bind _returnvalue (`KismetMathLibrary.RandomFloatInRange` 0.0 _spec))
  (bind (_output_x _output_y) (`KismetMathLibrary.BreakVector` (`|GetArrayItem` _vertex_2 _l_mid)))
  (bind (_output_x_2 _output_y_2 _output_z) (`KismetMathLibrary.BreakVector` (`|GetArrayItem` (`self.VERTEX`) (`local.L_SQ_B`))))
  (bind (_output_x_3 _output_y_3 _output_z_2) (`KismetMathLibrary.BreakVector` (`|GetArrayItem` (`self.VERTEX`) (`local.L_SQ_A`))))
  (bind (_output_x_4 _output_y_4 _output_z_3) (`KismetMathLibrary.BreakVector` (`|GetArrayItem` (`self.VERTEX`) (`local.L_SQ_B`))))
  (bind (_output_x_5 _output_y_5 _output_z_4) (`KismetMathLibrary.BreakVector` (`|GetArrayItem` (`self.VERTEX`) (`local.L_SQ_C`))))
  (bind (_output_x_6 _output_y_6 _output_z_5) (`KismetMathLibrary.BreakVector` (`|GetArrayItem` (`self.VERTEX`) (`local.L_SQ_D`))))
  (bind (_output_x_7 _output_y_7 _output_z_6) (`KismetMathLibrary.BreakVector` (`|GetArrayItem` (`self.VERTEX`) (`local.L_SQ_A`))))
  (bind (_output_x_8 _output_y_8 _output_z_7) (`KismetMathLibrary.BreakVector` (`|GetArrayItem` (`self.VERTEX`) (`local.L_SQ_C`))))
  (bind (_output_x_9 _output_y_9 _output_z_8) (`KismetMathLibrary.BreakVector` (`|GetArrayItem` (`self.VERTEX`) (`local.L_SQ_B`))))
  (bind (_output_x_10 _output_y_10 _output_z_9) (`KismetMathLibrary.BreakVector` (`|GetArrayItem` (`self.VERTEX`) (`local.L_SQ_D`))))
  (bind (_output_x_11 _output_y_11 _output_z_10) (`KismetMathLibrary.BreakVector` (`|GetArrayItem` (`self.VERTEX`) (`local.L_SQ_D`))))
  (bind (_output_x_12 _output_y_12 _output_z_11) (`KismetMathLibrary.BreakVector` (`|GetArrayItem` (`self.VERTEX`) (`local.L_SQ_A`))))
  (bind (_output_x_13 _output_y_13 _output_z_12) (`KismetMathLibrary.BreakVector` (`|GetArrayItem` (`self.VERTEX`) (`local.L_SQ_C`))))
  (bind _returnvalue_2 (/ (+ (- (`local.L_SQ_C`) (`local.L_SQ_A`)) 1) 2))
  (bind _returnvalue_3 (/ (+ _output_z_11 _output_z _output_z_12 _output_z_10) 4.0))
  (set `local.L_SQ_A` SQ_A)
  (set `local.L_SQ_B` SQ_B)
  (set `local.L_SQ_C` SQ_C)
  (set `local.L_SQ_D` SQ_D)
  (set `local.L_MID` (+ (`local.L_SQ_A`) (* (/ (- (`local.L_SQ_C`) (`local.L_SQ_A`)) 2) (+ (`self.Width`) 1))))
  ;[1 1 1] MID
  (`KismetArrayLibrary.Array_Set` _vertex_2 _l_mid (`KismetMathLibrary.MakeVector` _output_x _output_y (+ _returnvalue_3 _returnvalue)))
  (set `local.V_MID` (`KismetMathLibrary.Conv_IntToDouble` (`KismetMathLibrary.Or_IntInt` (`KismetMathLibrary.FTrunc` (- _returnvalue_3 _returnvalue)) (`KismetMathLibrary.FTrunc` (+ _returnvalue_3 (`KismetMathLibrary.RandomFloatInRange` 0.0 _spec))))))
  (set `self.SPEC` (/ (`self.SPEC`) 2.0))
  ;[1 1 1] Left
  (bind _output_get (set `local.L:_DMD_Left` (+ (`local.L_SQ_A`) _returnvalue_2)))
  (bind (_output_x_14 _output_y_14 _output_z_13) (`KismetMathLibrary.BreakVector` (`|GetArrayItem` _vertex_5 _output_get)))
  (`KismetArrayLibrary.Array_Set` _vertex_5 _output_get (`KismetMathLibrary.MakeVector` _output_x_14 _output_y_14 (select `bool` (== _output_z_13 0.0) :`false` _output_z_13 :`true` (+ (/ (+ _output_z_2 _output_z_4 (`local.V_MID`)) 3.0) (`KismetMathLibrary.RandomFloatInRange` 0.0 (`self.SPEC`))))))
  ;[1 1 1] Top
  (bind _output_get_2 (set `local.L_DMD_Top` (- (`local.L_MID`) _returnvalue_2)))
  (bind (_output_x_15 _output_y_15 _output_z_14) (`KismetMathLibrary.BreakVector` (`|GetArrayItem` _vertex_3 _output_get_2)))
  (`KismetArrayLibrary.Array_Set` _vertex_3 _output_get_2 (`KismetMathLibrary.MakeVector` _output_x_15 _output_y_15 (select `bool` (== _output_z_14 0.0) :`false` _output_z_14 :`true` (+ (/ (+ _output_z_6 _output_z_3 (`local.V_MID`)) 3.0) (`KismetMathLibrary.RandomFloatInRange` 0.0 (`self.SPEC`))))))
  ;[1 1 1] Right
  (bind _output_get_3 (set `local.L_DMD_Right` (+ (`local.L_SQ_B`) _returnvalue_2)))
  (bind (_output_x_16 _output_y_16 _output_z_15) (`KismetMathLibrary.BreakVector` (`|GetArrayItem` _vertex_4 _output_get_3)))
  (`KismetArrayLibrary.Array_Set` _vertex_4 _output_get_3 (`KismetMathLibrary.MakeVector` _output_x_16 _output_y_16 (select `bool` (== _output_z_15 0.0) :`false` _output_z_15 :`true` (+ (/ (+ _output_z_8 _output_z_5 (`local.V_MID`)) 3.0) (`KismetMathLibrary.RandomFloatInRange` 0.0 (`self.SPEC`))))))
  ;[1 1 1] Bottom
  (bind _output_get_4 (set `local.L_DMD_Bottom` (+ (`local.L_MID`) _returnvalue_2)))
  (bind (_output_x_17 _output_y_17 _output_z_16) (`KismetMathLibrary.BreakVector` (`|GetArrayItem` _vertex _output_get_4)))
  (`KismetArrayLibrary.Array_Set` _vertex _output_get_4 (`KismetMathLibrary.MakeVector` _output_x_17 _output_y_17 (select `bool` (== _output_z_16 0.0) :`false` _output_z_16 :`true` (+ (/ (+ _output_z_7 _output_z_9 (`local.V_MID`)) 3.0) (`KismetMathLibrary.RandomFloatInRange` 0.0 (`self.SPEC`))))))
  (return (`local.L_SQ_A`) (`local.L_SQ_B`) (`local.L_SQ_C`) (`local.L_SQ_D`) (`local.L_MID`) (`local.L:_DMD_Left`) (`local.L_DMD_Top`) (`local.L_DMD_Right`) (`local.L_DMD_Bottom`)))

(fn `GenerateLandscape`
  (params (`Polygon Size` :type Integer) (VertexNumbers :type Integer) (`UV scale` :type "Float (double-precision)") (LandscapeHeight :type "Float (double-precision)"))
  (`KismetArrayLibrary.Array_Clear` (`self.VERTEX`))
  (`KismetArrayLibrary.Array_Clear` (`self.TRIANGLES`))
  (`KismetArrayLibrary.Array_Clear` (`self.UV`))
  (`ProceduralMeshComponent.ClearAllMeshSections` (`self.ProceduralMesh`))
  (`self.GENERATOR` `Polygon Size` VertexNumbers `UV scale` LandscapeHeight)
  (`ProceduralMeshComponent.CreateMeshSection_LinearColor` :`self` (`self.ProceduralMesh`) :`Vertices` (`self.VERTEX`) :`Triangles` (`self.TRIANGLES`) :`UV0` (`self.UV`) :`bCreateCollision` true)
  (`PrimitiveComponent.SetMaterial` (`self.ProceduralMesh`) 0 "/Game/StarterContent/Materials/M_Ground_Moss.M_Ground_Moss"))

(fn `GENERATOR`
  (params (`Polygon Size` :type Integer) (VertexNumbers :type Integer) (`UV scale` :type "Float (double-precision)") (LandscapeHeight :type "Float (double-precision)"))
  (bind _vertex (`self.VERTEX`))
  (bind _vertex_2 (`self.VERTEX`))
  (bind _vertex_3 (`self.VERTEX`))
  (bind _sq_b (`self.SQ_B`))
  (bind _sq_c (`self.SQ_C`))
  (bind _sq_d (`self.SQ_D`))
  (bind _width (`self.Width`))
  (bind _width_2 (`self.Width`))
  (bind _counter_0 (`self.Counter_0`))
  (bind _counter_0_2 (`self.Counter_0`))
  (bind _counter_0_3 (`self.Counter_0`))
  (bind _counter_0_4 (`self.Counter_0`))
  (bind _vertex_4 (`self.VERTEX`))
  (bind _returnvalue (`KismetArrayLibrary.Array_Length` (`self.VERTEX`)))
  (bind _returnvalue_2 (- (`self.Width`) 1))
  (bind _returnvalue_3 (- (`self.Width`) 1))
  (bind (_output_x _output_y) (`KismetMathLibrary.BreakVector` (`|GetArrayItem` _vertex_4 _sq_d)))
  (bind (_output_x_2 _output_y_2) (`KismetMathLibrary.BreakVector` (`|GetArrayItem` _vertex _sq_c)))
  (bind (_output_x_3 _output_y_3) (`KismetMathLibrary.BreakVector` (`|GetArrayItem` _vertex_2)))
  (bind (_output_x_4 _output_y_4) (`KismetMathLibrary.BreakVector` (`|GetArrayItem` _vertex_3 _sq_b)))
  (set `self.SPEC` LandscapeHeight)
  (set `self.Width` (+ VertexNumbers 1))
  (`KismetArrayLibrary.Array_Clear` (`self.VERTEX`))
  (`KismetArrayLibrary.Array_Clear` (`self.TRIANGLES`))
  (for _index (range (+ _returnvalue_3 1))
    (for _index_2 (range (+ _returnvalue_3 1))
      (`|ExecutionSequence`
        (:`then_0`
          (`KismetArrayLibrary.Array_Add` (`self.VERTEX`) (`KismetMathLibrary.MakeVector` (`KismetMathLibrary.Conv_IntToDouble` (* _index `Polygon Size`)) (`KismetMathLibrary.Conv_IntToDouble` (* _index_2 `Polygon Size`)))))
        (:`then_1`
          (if (and (!= _index _returnvalue_2) (!= _index_2 _returnvalue_2))
            (bind _returnvalue_4 (+ _index_2 (* _index (`self.Width`))))
            (bind _returnvalue_5 (+ _index_2 (* (+ _index 1) (`self.Width`))))
            (`KismetProceduralMeshLibrary.ConvertQuadToTriangles` (`self.TRIANGLES`) _returnvalue_4 (+ _returnvalue_4 1) (+ _returnvalue_5 1) _returnvalue_5)))
        (:`then_2`
          (`KismetArrayLibrary.Array_Add` (`self.UV`) (`KismetMathLibrary.MakeVector2D` (* `UV scale` (* (`KismetMathLibrary.Conv_IntToDouble` _index) (/ 1.0 (`KismetMathLibrary.Conv_IntToDouble` (- _width 1))))) (* `UV scale` (* (`KismetMathLibrary.Conv_IntToDouble` _index_2) (/ 1.0 (`KismetMathLibrary.Conv_IntToDouble` (- _width 1)))))))))))
  (set `self.SQ_B` (- _returnvalue (`self.Width`)))
  (set `self.SQ_C` (- (`self.Width`) 1))
  (set `self.SQ_D` (- _returnvalue 1))
  (`KismetArrayLibrary.Array_Set` _vertex_2 0 (`KismetMathLibrary.MakeVector` _output_x_3 _output_y_3 (`KismetMathLibrary.RandomFloatInRange` 0.0 1000.0)))
  (`KismetArrayLibrary.Array_Set` _vertex_3 _sq_b (`KismetMathLibrary.MakeVector` _output_x_4 _output_y_4 (`KismetMathLibrary.RandomFloatInRange` 0.0 1000.0)))
  (`KismetArrayLibrary.Array_Set` _vertex _sq_c (`KismetMathLibrary.MakeVector` _output_x_2 _output_y_2 (`KismetMathLibrary.RandomFloatInRange` 0.0 1000.0)))
  (`KismetArrayLibrary.Array_Set` _vertex_4 _sq_d (`KismetMathLibrary.MakeVector` _output_x _output_y (`KismetMathLibrary.RandomFloatInRange` 0.0 1000.0)))
  (for _ (range (+ (* _width_2 (/ _width_2 4)) 1))
    (`KismetArrayLibrary.Array_Add` (`self.A`))
    (`KismetArrayLibrary.Array_Add` (`self.B`))
    (`KismetArrayLibrary.Array_Add` (`self.C`))
    (`KismetArrayLibrary.Array_Add` (`self.D`))
    (`KismetArrayLibrary.Array_Add` (`self.A_0`))
    (`KismetArrayLibrary.Array_Add` (`self.B_0`))
    (`KismetArrayLibrary.Array_Add` (`self.C_0`))
    (`KismetArrayLibrary.Array_Add` (`self.D_0`)))
  (`KismetArrayLibrary.Array_Set` (`self.A`) 1)
  (`KismetArrayLibrary.Array_Set` (`self.C`) 1 (`self.SQ_C`))
  (`KismetArrayLibrary.Array_Set` (`self.B`) 1 (`self.SQ_B`))
  (`KismetArrayLibrary.Array_Set` (`self.D`) 1 (`self.SQ_D`))
  (for _ (range 1 (+ (`KismetMathLibrary.FTrunc` (`KismetMathLibrary.Log` (`KismetMathLibrary.Conv_IntToDouble` (`self.Width`)) 2.0)) 1))
    (for _index_3 (range 1 (+ (`self.Counter`) 1))
      (bind (_a _b _c _d _mid _left _top _right _bottom) (`self.DIAMOND` (`|GetArrayItem` (`self.A`) _index_3) (`|GetArrayItem` (`self.B`) _index_3) (`|GetArrayItem` (`self.C`) _index_3) (`|GetArrayItem` (`self.D`) _index_3)))
      (`KismetArrayLibrary.Array_Set` (`self.A_0`) _counter_0_4 _a)
      (`KismetArrayLibrary.Array_Set` (`self.B_0`) _counter_0_4 _top)
      (`KismetArrayLibrary.Array_Set` (`self.C_0`) _counter_0_4 _left)
      (`KismetArrayLibrary.Array_Set` (`self.D_0`) _counter_0_4 _mid)
      (bind _result (`/Engine/EditorBlueprintResources/StandardMacros.IncrementInt` _counter_0_4)
        (:`  `
          (set `self.Counter_0` _result)
          (`KismetArrayLibrary.Array_Set` (`self.A_0`) _counter_0_3 _top)
          (`KismetArrayLibrary.Array_Set` (`self.B_0`) _counter_0_3 _b)
          (`KismetArrayLibrary.Array_Set` (`self.C_0`) _counter_0_3 _mid)
          (`KismetArrayLibrary.Array_Set` (`self.D_0`) _counter_0_3 _right)
          (bind _result_2 (`/Engine/EditorBlueprintResources/StandardMacros.IncrementInt` _counter_0_3)
            (:`  `
              (set `self.Counter_0` _result_2)
              (`KismetArrayLibrary.Array_Set` (`self.A_0`) _counter_0 _left)
              (`KismetArrayLibrary.Array_Set` (`self.B_0`) _counter_0 _mid)
              (`KismetArrayLibrary.Array_Set` (`self.C_0`) _counter_0 _c)
              (`KismetArrayLibrary.Array_Set` (`self.D_0`) _counter_0 _bottom)
              (bind _result_3 (`/Engine/EditorBlueprintResources/StandardMacros.IncrementInt` _counter_0)
                (:`  `
                  (set `self.Counter_0` _result_3)
                  (`KismetArrayLibrary.Array_Set` (`self.A_0`) _counter_0_2 _mid)
                  (`KismetArrayLibrary.Array_Set` (`self.B_0`) _counter_0_2 _right)
                  (`KismetArrayLibrary.Array_Set` (`self.C_0`) _counter_0_2 _bottom)
                  (`KismetArrayLibrary.Array_Set` (`self.D_0`) _counter_0_2 _d)
                  (bind _result_4 (`/Engine/EditorBlueprintResources/StandardMacros.IncrementInt` _counter_0_2)
                    (:`  `
                      (set `self.Counter_0` _result_4))))))))))
    (set `self.A` (`self.A_0`))
    (set `self.B` (`self.B_0`))
    (set `self.C` (`self.C_0`))
    (set `self.D` (`self.D_0`))
    (set `self.Counter_0` 1)
    (set `self.Counter` (* (`self.Counter`) 4)))
  (`KismetArrayLibrary.Array_Clear` (`self.A`))
  (`KismetArrayLibrary.Array_Clear` (`self.B`))
  (`KismetArrayLibrary.Array_Clear` (`self.C`))
  (`KismetArrayLibrary.Array_Clear` (`self.D`))
  (`KismetArrayLibrary.Array_Clear` (`self.A_0`))
  (`KismetArrayLibrary.Array_Clear` (`self.B_0`))
  (`KismetArrayLibrary.Array_Clear` (`self.C_0`))
  (`KismetArrayLibrary.Array_Clear` (`self.D_0`)))

(fn `UserConstructionScript`)