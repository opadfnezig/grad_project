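; Health pickup actor that restores health to the player's third-person character on contact.
; It spins around its yaw axis every Tick at RotationSpeed, scaled by delta time.
; When the sphere overlaps player 0's BP_ThirdPersonCharacter, it passes HealthPot to AddHealth, prints a message and destroys itself after a short delay.
; Nothing blocks repeat overlaps during that delay.
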(event `self.ReceiveTick`
  (params (DeltaSeconds :type "Float (single-precision)"))
  (`self.K2_AddActorWorldRotation` (`KismetMathLibrary.MakeRotator` 0.0 0.0 (* DeltaSeconds (`self.rotationSpeed`)))))

(event `self.Sphere.OnComponentBeginOverlap`
  (params (OverlappedComponent :type "PrimitiveComponent Object Reference") (OtherActor :type "Actor Object Reference") (OtherComp :type "PrimitiveComponent Object Reference") (OtherBodyIndex :type Integer) (bFromSweep :type Boolean) (SweepResult :type "HitResult Structure (by ref)"))
  (bind _asbp_third_person_character (cast `/Game/StarterContent/ThirdPerson/Blueprints/BP_ThirdPersonCharacter` (`GameplayStatics.GetPlayerCharacter` 0)))
  (if (== _asbp_third_person_character OtherActor)
    (`/Game/StarterContent/ThirdPerson/Blueprints/BP_ThirdPersonCharacter.AddHealth` _asbp_third_person_character (`self.HealthPot`))
    (`KismetSystemLibrary.PrintText` "HEALTH RECOVERED")
    (`KismetSystemLibrary.Delay` 0.32)
    (`self.K2_DestroyActor`)))

(fn `UserConstructionScript`)