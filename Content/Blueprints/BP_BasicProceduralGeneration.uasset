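; Actor Blueprint that generates a small random-height grass terrain with collision on a ProceduralMesh component at BeginPlay.
; GenerateLandscape clears previous data, calls GeneratingVertex, then creates the mesh section and applies the grass material.
; GeneratingVertex builds a square vertex grid with an independent random Z per vertex, converts each cell to triangles and spreads scaled UVs across the grid.
; No normals or tangents are supplied to the mesh.
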(event `self.ReceiveBeginPlay`
  (`self.GenerateLandscape` 10 64 12.0 64.0))

(fn `GenerateLandscape`
  (params (VertexCount :type Integer) (Size :type Integer) (UV_Scale :type "Float (double-precision)") (MaxHeight :type "Float (double-precision)"))
  (`KismetArrayLibrary.Array_Clear` (`self.VERTEX`))
  (`KismetArrayLibrary.Array_Clear` (`self.TRIANGLES`))
  (`KismetArrayLibrary.Array_Clear` (`self.UV`))
  (`ProceduralMeshComponent.ClearAllMeshSections` (`self.ProceduralMesh`))
  (`self.GeneratingVertex` VertexCount Size UV_Scale MaxHeight)
  (`ProceduralMeshComponent.CreateMeshSection_LinearColor` :`self` (`self.ProceduralMesh`) :`Vertices` (`self.Vertex`) :`Triangles` (`self.Triangles`) :`UV0` (`self.UV`) :`bCreateCollision` true)
  (`PrimitiveComponent.SetMaterial` (`self.ProceduralMesh`) 0 "/Game/StarterContent/Materials/M_Ground_Grass.M_Ground_Grass"))

(fn `GeneratingVertex`
  (params (VertexCount :type Integer) (Size :type Integer) (UV_Scale :type "Float (double-precision)") (MaxHeight :type "Float (double-precision)"))
  (bind _width (`self.Width`))
  (bind _returnvalue (- (`self.Width`) 1))
  (bind _returnvalue_2 (- (`self.Width`) 1))
  (set `self.Width` (+ VertexCount 1))
  (`KismetArrayLibrary.Array_Clear` (`self.VERTEX`))
  (`KismetArrayLibrary.Array_Clear` (`self.TRIANGLES`))
  (for _index (range (+ _returnvalue_2 1))
    (for _index_2 (range (+ _returnvalue_2 1))
      (`|ExecutionSequence`
        (:`then_0`
          (`KismetArrayLibrary.Array_Add` (`self.VERTEX`) (`KismetMathLibrary.MakeVector` (`KismetMathLibrary.Conv_IntToDouble` (* _index Size)) (`KismetMathLibrary.Conv_IntToDouble` (* _index_2 Size)) (`KismetMathLibrary.RandomFloatInRange` 0.0 MaxHeight))))
        (:`then_1`
          (if (and (!= _index _returnvalue) (!= _index_2 _returnvalue))
            (bind _returnvalue_3 (+ _index_2 (* _index (`self.Width`))))
            (bind _returnvalue_4 (+ _index_2 (* (+ _index 1) (`self.Width`))))
            (`KismetProceduralMeshLibrary.ConvertQuadToTriangles` (`self.TRIANGLES`) _returnvalue_3 (+ _returnvalue_3 1) (+ _returnvalue_4 1) _returnvalue_4)))
        (:`then_2`
          (`KismetArrayLibrary.Array_Add` (`self.UV`) (`KismetMathLibrary.MakeVector2D` (* (* _index (/ 1.0 (- _width 1))) UV_Scale) (* UV_Scale (* _index_2 (/ 1.0 (- _width 1)))))))))))

(fn `UserConstructionScript`)